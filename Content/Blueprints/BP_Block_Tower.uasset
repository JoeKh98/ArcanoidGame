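; BP_Block_Tower is a destructible tower block that awards points to the game mode's score when it fractures.
; BeginPlay caches BP_GameMode; on fracture, the block enables gravity, changes collision responses and applies a radial impulse from above its center.
; It then plays a collapse sound, updates the score and destroys itself after a short delay.
; The construction script is empty, leaving block color material logic unconnected.
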(event OnComponentFracture(Destructible)
  (params (HitPoint :type Vector%20%28by%20ref%29 :default "0, 0, 0") (HitDirection :type Vector%20%28by%20ref%29 :default "0, 0, 0"))
  (bind _destructible (Variables|Default|GetDestructible))
  (bind _returnvalue (Transformation|GetWorldLocation _destructible))
  (Physics|SetEnableGravity (Variables|Default|GetDestructible) true)
  (Collision|SetCollisionResponsetoChannel (Variables|Default|GetDestructible) "ECC_PhysicsBody" "ECR_Ignore")
  (Collision|SetCollisionResponsetoChannel (Variables|Default|GetDestructible) "ECC_Destructible" "ECR_Block")
  (Collision|SetCollisionResponsetoChannel (Variables|Default|GetDestructible) "ECC_WorldStatic" "ECR_Block")
  (Physics|AddRadialImpulse _destructible (Math|Vector|MakeVector (.x _returnvalue) (.y _returnvalue) (+ (.z _returnvalue) 1e+02)) 4e+01 1e+04 "RIF_Constant" false)
  (Audio|SpawnSound2D "/Game/StarterContent/Audio/Collapse02.Collapse02" 1.0 1.0 0.0 0)
  (Default|UpdateScore (Variables|Default|GetGameMode) (Variables|Default|GetPoints))
  (Utilities|FlowControl|Delay 1.5)
  (Actor|DestroyActor))

(event EventBeginPlay
  (bind _asbp_game_mode (Utilities|Casting|CastToBP_GameMode (Game|GetGameMode)))
  (Variables|Default|SetGameMode _asbp_game_mode))

(fn ConstructionScript)