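; BP_Pawn is the player's paddle pawn in a ball-and-paddle game, handling ball spawning, launching and movement.
; On BeginPlay it caches BP_GameMode, then NewBall spawns a BP_Ball at the Arrow component's location unless the game is over.
; Shoot input launches the stored ball if it is inactive, and Exit quits the game.
; The Move axis slides the Player component along world X, scaled by Speed and clamped to fixed bounds.
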(event Custom|NewBall
  ;[1 1 1] Spawn a ball
  (if (not (Variables|/Game/GameMode/BP_GameMode.BP_GameMode_C|GetisGameOver (Variables|Default|GetGameMode)))
    (bind _returnvalue (Game|SpawnActorfromClass "/Game/Blueprints/BP_Ball.BP_Ball_C" (Math|Transform|MakeTransform (.location (Transformation|GetWorldTransform (Variables|Default|GetArrow))) "0, 0, 0" "1,1,1") "Undefined" 0 0))
    (Variables|Default|SetBall _returnvalue)))

(event EventBeginPlay
  ;[1 1 1] Getting a GameMode
  (bind _asbp_game_mode (Utilities|Casting|CastToBP_GameMode (Game|GetGameMode)))
  (Variables|Default|SetGameMode _asbp_game_mode)
  (CallFunction|NewBall))

(event Input|ActionEvents|InputActionShoot
  (params (Key :type Key%20Structure :default "None"))
  (bind _ball (Variables|Default|GetBall))
  ;[1 1 1] Fire Ball event SPACEBAR
  (:Pressed
    (if (and (Utilities|IsValid _ball) (not (Variables|/Game/Blueprints/BP_Ball.BP_Ball_C|GetisActive _ball)))
      (Default|LaunchBall (Variables|Default|GetBall)))))

(event Input|ActionEvents|InputActionExit
  (params (Key :type Key%20Structure :default "None"))
  (:Pressed
    (Game|QuitGame 0 "Quit" false)))

(event Input|AxisEvents|InputAxisMove
  (params (AxisValue :type Float%20%28single-precision%29))
  (bind _player (Variables|Default|GetPlayer))
  (bind _returnvalue (Transformation|GetWorldLocation _player))
  ;[1 1 1] Paddle Movement
  (Transformation|SetWorldLocation (Variables|Default|GetPlayer) (Math|Vector|MakeVector (Math|Float|Clamp(Float) (+ (.x _returnvalue) (* AxisValue (Variables|Default|GetSpeed))) -1.08e+03 1.08e+03) (.y _returnvalue) (.z _returnvalue)) false false))

(fn ConstructionScript)