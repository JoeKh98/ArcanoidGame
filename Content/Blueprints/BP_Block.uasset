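; BP_Block is a block that is destroyed when a ball hits it and awards its points to the score.
; It caches BP_GameMode on BeginPlay, then on a BP_Ball hit destroys itself and passes Points to the game mode's UpdateScore.
; The construction script is empty; its nodes for tinting a dynamic M_Ball material with BlockColor are disconnected and never run.
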(event OnComponentHit(Block)
  (params (HitComponent :type Primitive%20Component%20Object%20Reference) (OtherActor :type Actor%20Object%20Reference) (OtherComp :type Primitive%20Component%20Object%20Reference) (NormalImpulse :type Vector :default "0, 0, 0") (Hit :type Hit%20Result%20Structure%20%28by%20ref%29))
  (Utilities|Casting|CastToBP_Ball OtherActor)
  (Actor|DestroyActor)
  (Default|UpdateScore (Variables|Default|GetGameMode) (Variables|Default|GetPoints)))

(event EventBeginPlay
  (bind _asbp_game_mode (Utilities|Casting|CastToBP_GameMode (Game|GetGameMode)))
  (Variables|Default|SetGameMode _asbp_game_mode))

(fn ConstructionScript)