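; Game mode for a block-clearing game that tracks score, lives and the win and loss states.
; On BeginPlay it creates the HUD and resets the session, then pushes score and life changes to the widget.
; Losing a life costs points, with the score floored at zero, and a check counts actors tagged "block" to detect a clear.
; Game over and level clear each play a sound, then reload Main_Level after a delay.
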(event Custom|Reset
  (bind _maxlives (Variables|Default|GetMaxLives))
  ;[1 1 1] Reset Game
  (Variables|Default|SetLives _maxlives)
  (Variables|/Game/Blueprints/Widgets/WBP_HUD.WBP_HUD_C|SetLives (Variables|Default|GetHUD) _maxlives)
  (Variables|Default|SetCurrentPoints 0)
  (Variables|/Game/Blueprints/Widgets/WBP_HUD.WBP_HUD_C|SetPoints (Variables|Default|GetHUD) 0)
  (Variables|Default|SetCurrentPoints 0)
  (Variables|Default|SetisGameOver false))

(event Custom|UpdateScore
  (params (Points :type Integer))
  ;[1 1 1] Update Score
  (if (<= (+ (Variables|Default|GetCurrentPoints) Points) 0)
    (Variables|Default|SetCurrentPoints 0)
    (else
      (Variables|Default|SetCurrentPoints (+ (Variables|Default|GetCurrentPoints) Points))))
  (Variables|/Game/Blueprints/Widgets/WBP_HUD.WBP_HUD_C|SetPoints (Variables|Default|GetHUD) (Variables|Default|GetCurrentPoints)))

(event Custom|LifeLost
  ;[1 1 1] LifeLost
  (CallFunction|UpdateScore -500)
  (if (<= (Variables|Default|GetLives) 0)
    (CallFunction|GameOver)
    (else
      (bind _result (Math|Integer|DecrementInt (Variables|Default|GetLives))
        (:%20%20
          (Variables|/Game/Blueprints/Widgets/WBP_HUD.WBP_HUD_C|SetLives (Variables|Default|GetHUD) _result))))))

(event Custom|GameOver
  ;[1 1 1] GameOver
  (Variables|Default|SetisGameOver true)
  (Audio|PlaySound2D "/Game/Audio/GameOver.GameOver" 1.0 1.0 0.0 0 0)
  (Utilities|FlowControl|Delay 5.0)
  (Game|OpenLevel(byName) "Main_Level"))

(event Custom|BlocksRamainingCheck
  ;[1 1 1] Blocks Remaining Check
  (bind _outactors (Actor|GetAllActorswithTag "block"))
  (Variables|Default|SetBlocksRemaining (Utilities|Array|Length _outactors))
  (if (<= (Variables|Default|GetBlocksRemaining) 0)
    (CallFunction|LevelClear)))

(event Custom|LevelClear
  ;[1 1 1] Level Clear
  (Variables|Default|SetbIsLevelClear true)
  (Audio|PlaySound2D "/Game/Audio/Win.Win" 1.0 1.0 0.0 0 0)
  (Utilities|FlowControl|Delay 5.0)
  (Game|OpenLevel(byName) "Main_Level"))

(event EventBeginPlay
  ;[1 1 1] Add HUD
  (bind _returnvalue (UserInterface|CreateWidget "/Game/Blueprints/Widgets/WBP_HUD.WBP_HUD_C"))
  (bind _output_get (Variables|Default|SetHUD _returnvalue))
  (UserInterface|Viewport|AddtoViewport _output_get 0)
  (CallFunction|Reset))

(fn ConstructionScript)